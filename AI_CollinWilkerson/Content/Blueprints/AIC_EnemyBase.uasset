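; Base enemy AI controller that runs BT_Enemy after a short possession delay and starts in Patrol.
; Perception updates check sight, hearing and damage per actor through OnDetect, then write state, target and point of interest to the Blackboard.
; Sighting any actor during Patrol triggers Attack; sighting the player always does.
; Noise or damage during Patrol or Investigate sets Investigate at the stimulus location.
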(event `self.ReceivePossess`
  (params (PossessedPawn :type "Pawn Object Reference"))
  (`KismetSystemLibrary.Delay` 0.2)
  (`self.RunBehaviorTree` "/Game/BehaviorTrees/BT_Enemy.BT_Enemy")
  (`self.SetTarget` null)
  (`self.SetState` "NewEnumerator0"))

(event `self.AIPerception.OnPerceptionUpdated`
  (params (UpdatedActors :type "Array of Actor Object Reference (by ref)"))
  (for _array_element UpdatedActors
    (`|ExecutionSequence`
      (:`then_0`
        (bind _detected (`self.OnDetect` _array_element "NewEnumerator1"))
        (if _detected
          (`self.HandleSenseSight` _array_element)
          (if (== _array_element (`GameplayStatics.GetPlayerCharacter` 0))
            (`self.GetState`)
            (switch `/Game/BehaviorTrees/E_EnemyStates` "NewEnumerator0"
              (:`NewEnumerator0`
                _)
              (:`NewEnumerator2`
                _))
            (`self.SetTarget` _array_element)
            (`self.SetState` "NewEnumerator1"))))
      (:`then_1`
        (bind (_detected_2 _stimulus) (`self.OnDetect` _array_element "NewEnumerator2"))
        (if _detected_2
          (`KismetSystemLibrary.PrintString` "heard")
          (bind _returnvalue (`self.GetState`))
          (switch `/Game/BehaviorTrees/E_EnemyStates` _returnvalue
            (:`NewEnumerator0`
              _)
            (:`NewEnumerator2`
              _))
          (`self.SetState` "NewEnumerator2")
          (`BlackboardComponent.SetValueAsVector` (`self.Blackboard`) (`self.POIKey`) (`.StimulusLocation` (break `AIStimulus` _stimulus)))))
      (:`then_2`
        (bind (_detected_3 _stimulus_2) (`self.OnDetect` _array_element "NewEnumerator3"))
        (if _detected_3
          (`KismetSystemLibrary.PrintString` "damaged")
          (bind _returnvalue_2 (`self.GetState`))
          (switch `/Game/BehaviorTrees/E_EnemyStates` _returnvalue_2
            (:`NewEnumerator0`
              _)
            (:`NewEnumerator2`
              _))
          (`self.SetState` "NewEnumerator2")
          (`BlackboardComponent.SetValueAsVector` (`self.Blackboard`) (`self.POIKey`) (`.StimulusLocation` (break `AIStimulus` _stimulus_2))))))))

(fn `GetState`
  (returns (ReturnValue :type "/Game/BehaviorTrees/E_EnemyStates Enum"))
  (return (cast `/Game/BehaviorTrees/E_EnemyStates` (`BlackboardComponent.GetValueAsEnum` (`self.Blackboard`) (`self.StateKey`)))))

(fn `HandleSenseSight`
  (params (ObjectValue :type "Object Object Reference"))
  (bind _returnvalue (`self.GetState`))
  (if true
    (switch `/Game/BehaviorTrees/E_EnemyStates` _returnvalue
      (:`NewEnumerator0`
        (`self.SetTarget` ObjectValue)
        (`self.SetState` "NewEnumerator1")))))

(fn `OnDetect`
  (params (Actor :type "Actor Object Reference") (Senses :type "/Game/Enum/E_Senses Enum" :default "NewEnumerator0"))
  (returns (Detected :type Boolean) (Stimulus :type "AIStimulus Structure"))
  (bind _info (`AIPerceptionComponent.GetActorsPerception` (`self.AIPerception`) Actor))
  (for _array_element (`.LastSensedStimuli` (break `ActorPerceptionBlueprintInfo` _info))
    (bind _returnvalue (`AIPerceptionSystem.GetSenseClassForStimulus` _array_element))
    (if (== _returnvalue (select `/Game/Enum/E_Senses` Senses :`NewEnumerator1` "/Script/AIModule.AISense_Sight" :`NewEnumerator2` "/Script/AIModule.AISense_Hearing" :`NewEnumerator3` "/Script/AIModule.AISense_Damage" :!type "Object Class Reference"))
      (return (`.bSuccessfullySensed` (break `AIStimulus` _array_element)) _array_element))))

(fn `SetState`
  (params (Enum :type "/Game/BehaviorTrees/E_EnemyStates Enum" :default "NewEnumerator0"))
  (`BlackboardComponent.SetValueAsEnum` (`self.Blackboard`) (`self.StateKey`) Enum))

(fn `SetTarget`
  (params (ObjectValue :type "Object Object Reference"))
  (`BlackboardComponent.SetValueAsObject` (`self.Blackboard`) (`self.AttackKey`) ObjectValue))

(fn `UserConstructionScript`)