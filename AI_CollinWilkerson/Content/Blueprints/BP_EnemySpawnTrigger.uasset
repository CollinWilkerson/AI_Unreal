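; Trigger volume that spawns waves of enemies once the player pawn overlaps its box.
; The overlap sets a three-second timer that calls SpawnEnemies, which fills every spawn point with a randomly chosen BP_EnemyCharacter or BP_RifleEnemy and increments the wave count.
; The timer's looping flag compares waves spawned to the total only when set, so a looping timer never stops at that limit.
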(event `self.Box.OnComponentBeginOverlap`
  (params (OverlappedComponent :type "PrimitiveComponent Object Reference") (OtherActor :type "Actor Object Reference") (OtherComp :type "PrimitiveComponent Object Reference") (OtherBodyIndex :type Integer) (bFromSweep :type Boolean) (SweepResult :type "HitResult Structure (by ref)"))
  (if (== OtherActor (`GameplayStatics.GetPlayerPawn` 0))
    (`KismetSystemLibrary.K2_SetTimerDelegate` (delegate `SpawnEnemies`) 3.0 (< (`self.WavesSpawned`) (`self.TotalWaves`)))))

(event `SpawnEnemies`
  (for _index (range (+ (+ (`KismetArrayLibrary.Array_Length` (`self.SpawnPoints`)) -1) 1))
    (if (`KismetMathLibrary.RandomBool`)
      (bind _output (`|GetArrayItem` (`self.SpawnPoints`) _index))
      (`|SpawnActorFromClass` "/Game/ThirdPerson/Blueprints/BP_EnemyCharacter.BP_EnemyCharacter_C" _output "Undefined" "MultiplyWithRoot" null null)
      (else
        (`|SpawnActorFromClass` "/Game/ThirdPerson/Blueprints/BP_RifleEnemy.BP_RifleEnemy_C" _output "Undefined" "MultiplyWithRoot" null null))))
  (set `self.WavesSpawned` (+ (`self.WavesSpawned`) 1)))

(fn `UserConstructionScript`)